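; BP_Heal is a health pickup for the shooting game that players collect by interacting with it.
; On Interact, the server adds a fixed heal amount through the interacting character's BP_ShootingPlayerState, then destroys the pickup.
; When focused, it highlights its static mesh through custom depth rendering, and ShowInfo puts a recovery prompt on the HUD.
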(event EventShowOutline
  (params (bIsFocus :type Boolean))
  (Rendering|SetRenderCustomDepth (Variables|Default|GetStaticMesh) bIsFocus))

(event EventShowInfo
  (params (HUD :type Interaction%20Widget%20Object%20Reference))
  (Utilities|IsValid HUD
    (:Is%20Valid
      (Default|SetInfoText HUD "Press [E] to recover HP"))))

(event EventInteract
  (params (InteractTarget :type Actor%20Object%20Reference))
  (Networking|SwitchHasAuthority
    (:Authority
      (bind _assystem_char (Utilities|Casting|CastToSystemChar InteractTarget))
      (bind _asbp_shooting_player_state (Utilities|Casting|CastToBP_ShootingPlayerState (Variables|/Script/Engine.Pawn|GetPlayerState _assystem_char)))
      (Default|AddHeal _asbp_shooting_player_state 5e+01)
      (Actor|DestroyActor))))

(fn ConstructionScript)